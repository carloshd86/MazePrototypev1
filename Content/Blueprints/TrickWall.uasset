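; TrickWall is a wall actor whose static mesh moves along its local Z axis when triggered.
; ActivateWall fires only once, playing a timeline whose track sets a per-update offset that accumulates, so total travel depends on tick count.
; BeginPlay caches the player controller and the first WeepingAngel in the level, though neither reference is used in these graphs.
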(event Custom|ActivateWall
  (if (not (Variables|Default|GetisActivated))
    (Variables|Default|SetisActivated true)
    (bind _newtrack_0 (Timeline|Timeline_0 Play)
      (:Update
        (Transformation|AddLocalOffset (Variables|Debug|GetStaticMeshComponent) (Math|Vector|MakeVector 0.0 0.0 (Math|Float|Lerp 0.0 6.0 _newtrack_0)) false false)))))

(event EventBeginPlay
  (Variables|Default|SetPlayerRef (Game|GetPlayerController 0))
  (bind _outactors (Actor|GetAllActorsOfClass "/Game/ThirdPersonBP/Blueprints/WeepingAngel.WeepingAngel_C"))
  (Variables|Default|SetWeepingAngelRef (Utilities|Array|Get(acopy) _outactors)))

(fn ConstructionScript)